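; BP_Inventory_Slot is an inventory slot for grabbable items, built around a motion controller component.
; Its sphere overlaps track the current BP_Inventory_Item_Class actor, clearing it when that item leaves.
; The Put event checks that the passed grab component belongs to that item, then calls TryGrab with the slot's MotionController to hold it.
; It also moves the item to the controller's location and sets its mesh to overlap Pawns.
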(event OnComponentBeginOverlap(Sphere)
  (params (OverlappedComponent :type Primitive%20Component%20Object%20Reference) (OtherActor :type Actor%20Object%20Reference) (OtherComp :type Primitive%20Component%20Object%20Reference) (OtherBodyIndex :type Integer) (bFromSweep :type Boolean) (SweepResult :type Hit%20Result%20Structure%20%28by%20ref%29))
  (bind _asbp_inventory_item_class (Utilities|Casting|CastToBP_Inventory_Item_Class OtherActor))
  (Variables|Default|SetItemInSlot _asbp_inventory_item_class)
  (Development|PrintString "Added item slot"))

(event OnComponentEndOverlap(Sphere)
  (params (OverlappedComponent :type Primitive%20Component%20Object%20Reference) (OtherActor :type Actor%20Object%20Reference) (OtherComp :type Primitive%20Component%20Object%20Reference) (OtherBodyIndex :type Integer))
  (bind _asbp_inventory_item_class (Utilities|Casting|CastToBP_Inventory_Item_Class OtherActor))
  (if (== _asbp_inventory_item_class (Variables|Default|GetItemInSlot))
    (Variables|Default|SetItemInSlot 0)
    (Development|PrintString "Removed item slot")))

(event Custom|Put
  (params (GrabComponent :type Grab%20Component%20Object%20Reference))
  (bind _iteminslot (Variables|Default|GetItemInSlot))
  (bind _motioncontroller (Variables|Default|GetMotionController))
  (Utilities|IsValid _iteminslot
    (:Is%20Valid
      (if (== GrabComponent (Variables|/Game/MyContent/Class/BP_Interaction_Class.BP_Interaction_Class_C|GetGrabComponent _iteminslot))
        (Default|TryGrab (Variables|/Game/MyContent/Class/BP_Interaction_Class.BP_Interaction_Class_C|GetGrabComponent _iteminslot) _motioncontroller)
        (Transformation|SetActorLocation (Variables|Default|GetItemInSlot) (Transformation|GetWorldLocation _motioncontroller) false false)
        (Collision|SetCollisionResponsetoChannel (Actor|GetComponentbyClass (.AsBP%20Inventory%20Item%20Class (Utilities|Casting|CastToBP_Inventory_Item_Class (Components|GetOwner (Variables|/Game/MyContent/Class/BP_Interaction_Class.BP_Interaction_Class_C|GetGrabComponent _iteminslot)))) "/Script/Engine.StaticMeshComponent") "ECC_Pawn" "ECR_Overlap")
        (Development|PrintString "Put to Inventoryy")))))

(event EventBeginPlay)

(event Collision|EventActorBeginOverlap
  (params (OtherActor :type Actor%20Object%20Reference)))

(event EventTick
  (params (DeltaSeconds :type Float%20%28single-precision%29)))

(fn ConstructionScript)